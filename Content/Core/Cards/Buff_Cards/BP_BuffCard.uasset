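; BP_BuffCard is a buff card that heals the player when played.
; OnCardPlay takes the card's Power as Value and passes itself to the player AnimBP's LargeSpell, deferring the effect until AnimationCallback.
; The callback calls OnApply, which adds Value to CurrentHealth and starts a one-shot timer whose end event only prints debug text.
; A separate HealingBuff function repeats the health addition but is not called here.
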(event `/Game/Core/Cards/Basic_Cards/CardInterface.onCardPlay`
  (bind (_card_name _card_description _card_uses _card_element _card_rarity _card_image _card_blueprintclass _card_cardtype _card_power) (break `/Game/Core/Cards/S_CardStructure` (`/Game/Core/UI/W_Card.Card` (`self.CardWidget`))))
  (set `self.value` _card_power)
  (bind _asabp_player (cast `/Game/Core/Animations/ABP_Player` (`SkeletalMeshComponent.GetAnimInstance` (`Character.Mesh` (`GameplayStatics.GetPlayerCharacter` 0)))))
  (`/Game/Core/Animations/ABP_Player.largeSpell` _asabp_player self))

(event `onApply`
  (bind _asbp_player (cast `/Game/Core/Character/Player/BP_Player` (`GameplayStatics.GetPlayerCharacter` 0)))
  (set `/Game/Core/Character/BP_BaseCharacter.CurrentHealth` (+ (`self.value`) (`/Game/Core/Character/BP_BaseCharacter.CurrentHealth` _asbp_player)) _asbp_player)
  (`KismetSystemLibrary.K2_SetTimerDelegate` (delegate `onTimerEnd`) (`KismetMathLibrary.Conv_IntToDouble` (`self.timer`))))

(event `onTimerEnd`
  (cast `/Game/Core/Character/Player/BP_Player` (`GameplayStatics.GetPlayerCharacter` 0)
    (:`then`
      _)
    (:`CastFailed`
      _))
  (`KismetSystemLibrary.PrintString` "Hello"))

(event `/Game/Core/Cards/Basic_Cards/CardInterface.animationCallback`
  (`KismetSystemLibrary.PrintString` "wuhuu")
  (`self.onApply`))

(fn `HealingBuff`
  (bind _asbp_player (cast `/Game/Core/Character/Player/BP_Player` (`GameplayStatics.GetPlayerCharacter` 0)))
  (set `/Game/Core/Character/BP_BaseCharacter.CurrentHealth` (+ (`/Game/Core/Character/BP_BaseCharacter.CurrentHealth` _asbp_player) (`self.value`)) _asbp_player))

(fn `UserConstructionScript`
  (`parent.UserConstructionScript`))