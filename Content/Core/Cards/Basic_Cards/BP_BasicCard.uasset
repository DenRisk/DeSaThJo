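; BP_BasicCard is the base Blueprint for playable cards, handling cooldown gating and routing play to damage or buff cards.
; BeforePlay refuses a play while the CardWidget timer bar is above zero, otherwise it starts the cooldown, so the UI progress bar serves as cooldown state.
; OnCardPlayEnd switches on card type and casts itself to BP_DamageCard or BP_BuffCard to call OnCardPlay, which is empty here.
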(event `/Game/Core/Cards/Basic_Cards/CardInterface.OnCardPlayEnd`
  (switch `/Game/Core/Cards/Basic_Cards/EnumCardType` "NewEnumerator0"
    (:`NewEnumerator0`
      (bind _asbp_damage_card (cast `/Game/Core/Cards/DMG_Cards/BP_DamageCard` self))
      (`self.onCardPlay` _asbp_damage_card))
    (:`NewEnumerator1`
      (bind _asbp_buff_card (cast `/Game/Core/Cards/Buff_Cards/BP_BuffCard` self))
      (`self.onCardPlay` _asbp_buff_card))))

(event `/Game/Core/Cards/Basic_Cards/CardInterface.onCardPlay`)

(fn `beforePlay`
  (returns (cardPlayed :type Boolean))
  (bind _timeractive (`self.checkIfTimerActive`))
  (if _timeractive
    (return false)
    (else
      (`/Game/Core/UI/W_Card.StartCooldown` (`self.CardWidget`) (`self.Cooldown`))
      (return true))))

(fn `checkIfTimerActive`
  (returns (timerActive :type Boolean))
  (bind _percent (`ProgressBar.Percent` (`/Game/Core/UI/W_Card.TimerProgressBar` (`self.CardWidget`))))
  (`KismetSystemLibrary.PrintString` (`KismetStringLibrary.Conv_DoubleToString` _percent))
  (return (> _percent 0.0)))

(fn `UserConstructionScript`)