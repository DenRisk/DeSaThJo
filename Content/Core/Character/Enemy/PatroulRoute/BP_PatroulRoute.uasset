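; BP_PatroulRoute is an enemy patrol route that supplies world-space waypoints from the points of its PatroulRoute spline.
; IncrementPatroulRoute steps PatroulIndex by Direction, setting Direction to -1 at the last point and 1 at the first for back-and-forth traversal.
; GetSplinePointAsWorldPosition returns the world location of the spline point at the current index.
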(event `IncrementPatroulRoute`
  (bind _output_get (set `self.PatroulIndex` (+ (`self.PatroulIndex`) (`self.Direction`))))
  (if (== _output_get (- (`SplineComponent.GetNumberOfSplinePoints` (`self.PatroulRoute`)) 1))
    (set `self.Direction` -1)
    (elif (== (`self.PatroulIndex`) 0)
      (set `self.Direction` 1))))

(fn `GetSplinePointAsWorldPosition`
  (returns (Location :type "Vector Structure"))
  (return (`SplineComponent.GetLocationAtSplinePoint` (`self.PatroulRoute`) (`self.PatroulIndex`) "World")))

(fn `UserConstructionScript`)