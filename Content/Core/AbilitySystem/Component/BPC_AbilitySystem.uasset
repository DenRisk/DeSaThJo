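; BPC_AbilitySystem is an ability component that launches lava ball projectiles for its owner and applies their damage on impact.
; SpawnProjectile spawns a BP_Projectile_Lavaball toward a target, binds its impact event and makes its collision ignore the owner while moving.
; On impact it sends the damage info to the hit actor, reports the damage to AI perception and broadcasts OnAttackEnded.
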(event `self.ReceiveBeginPlay`
  (set `self.Owner` (`self.GetOwner`)))

(event `SpawnProjectile`
  (params (SpawnTransform :type "Transform Structure") (Target :type "Actor Object Reference") (DamageInfo :type "/Game/Core/DamageSystem/Structure/STR_DamageInfo Structure") (Owner :type "/Game/Core/Character/Player/BP_Player Object Reference"))
  (if (== (`GameplayStatics.GetObjectClass` (`self.Owner`)) "/Game/Core/Cards/DMG_Cards/BP_DamageCard.BP_DamageCard_C")
    (set `self.Owner` Owner))
  (bind _returnvalue (`|SpawnActorFromClass` "/Game/Core/AbilitySystem/Projectiles/Actors/BP_Projectile_Lavaball.BP_Projectile_Lavaball_C" SpawnTransform "Undefined" "MultiplyWithRoot" (`self.Owner`) 1000.0 0.0 Target false null))
  (add `/Game/Core/AbilitySystem/Projectiles/BP_Projectile_Base.OnProjectileImpact` _returnvalue (delegate `OnProjectileHit`))
  (`PrimitiveComponent.IgnoreActorWhenMoving` (`/Game/Core/AbilitySystem/Projectiles/BP_Projectile_Base.BoxCollision` _returnvalue) (`self.Owner`) true))

(event `OnProjectileHit`
  (params (OtherActor :type "Actor Object Reference") (Hit :type "HitResult Structure"))
  (bind _owner (`self.Owner`))
  (message `/Game/Core/DamageSystem/Interface/BPI_Damageable.TakeDamage` OtherActor (stale `SpawnProjectile` DamageInfo) _owner)
  (`AISense_Damage.ReportDamageEvent` OtherActor _owner (`.Amount_2_875E54C14825CA53868FBCBEAA26AC07` (break `/Game/Core/DamageSystem/Structure/STR_DamageInfo` (stale `SpawnProjectile` DamageInfo))) (`Actor.K2_GetActorLocation` (`self.Owner`)))
  (`self.OnAttackEnded`))